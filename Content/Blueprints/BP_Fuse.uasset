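; BP_Fuse is a pickup that gives the player a fuse for an electrical panel.
; Its box trigger enables input and shows an on-screen prompt while a shooter character overlaps it, then disables input when any overlap ends.
; Pressing E fires once, marking the fuse as taken and setting HasFuse on the referenced ElectricalPanelBlueprint.
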(event `self.BoxTrigger.OnComponentBeginOverlap`
  (params (OverlappedComponent :type "PrimitiveComponent Object Reference") (OtherActor :type "Actor Object Reference") (OtherComp :type "PrimitiveComponent Object Reference") (OtherBodyIndex :type Integer) (bFromSweep :type Boolean) (SweepResult :type "HitResult Structure (by ref)"))
  ; Interaction Logic
  (cast `/Game/Variant_Shooter/Blueprints/BP_ShooterCharacter` OtherActor)
  (`self.EnableInput` (`GameplayStatics.GetPlayerController` 0))
  (if (not (`self.Interacted`))
    (`KismetSystemLibrary.PrintString` "PRESS E TO INTERACT" true true (struct :`R` 1.0 :`G` 1.0 :`B` 1.0 :`A` 1.0) 2.0 "Interact")))

(event `self.BoxTrigger.OnComponentEndOverlap`
  (params (OverlappedComponent :type "PrimitiveComponent Object Reference") (OtherActor :type "Actor Object Reference") (OtherComp :type "PrimitiveComponent Object Reference") (OtherBodyIndex :type Integer))
  ; Interaction Logic
  (`self.DisableInput` (`GameplayStatics.GetPlayerController` 0)))

(event `Key|E`
  (params (Key :type "Key Structure"))
  ; Interaction Logic
  (:`Pressed`
    (`/Engine/EditorBlueprintResources/StandardMacros.DoOnce` false
      (:`Completed`
        (set `self.Interacted` true)
        (`KismetSystemLibrary.PrintString` "FUSE TAKEN")
        (set `/Game/Blueprints/BP_ElectricalPanel.HasFuse` true (`self.ElectricalPanelBlueprint`))))))

(fn `UserConstructionScript`)