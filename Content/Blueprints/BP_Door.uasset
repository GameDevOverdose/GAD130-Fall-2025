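; BP_Door is an interactive door actor that swings open and closed when the player presses E nearby.
; A box trigger enables player input on overlap and disables it on exit.
; E and the OpenDoor event share a FlipFlop that plays or reverses a timeline, which interpolates the door's yaw between closed and a quarter turn.
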(event `self.BoxTrigger.OnComponentBeginOverlap`
  (params (OverlappedComponent :type "PrimitiveComponent Object Reference") (OtherActor :type "Actor Object Reference") (OtherComp :type "PrimitiveComponent Object Reference") (OtherBodyIndex :type Integer) (bFromSweep :type Boolean) (SweepResult :type "HitResult Structure (by ref)"))
  (`self.EnableInput` (`GameplayStatics.GetPlayerController` 0)))

(event `self.BoxTrigger.OnComponentEndOverlap`
  (params (OverlappedComponent :type "PrimitiveComponent Object Reference") (OtherActor :type "Actor Object Reference") (OtherComp :type "PrimitiveComponent Object Reference") (OtherBodyIndex :type Integer))
  (`self.DisableInput` (`GameplayStatics.GetPlayerController` 0)))

(event `Key|E`
  (params (Key :type "Key Structure"))
  (:`Pressed`
    (`/Engine/EditorBlueprintResources/StandardMacros.FlipFlop` :!label _label
      (:`A`
        (bind (_direction _value) (`Timeline|Open Door` :!label _label_2)
          (:`Update`
            (bind (_returnvalue_x _returnvalue_y _returnvalue_z) (`KismetMathLibrary.BreakVector` (`KismetMathLibrary.VLerp` (0.0 0.0 0.0) (0.0 0.0 90.0) _value)))
            (`SceneComponent.K2_SetRelativeRotation` (`self.Door`) (`KismetMathLibrary.MakeRotator` 0.0 0.0 _returnvalue_z) false false))))
      (:`B`
        (goto _label_2 :!via `Reverse`)))))

(event `OpenDoor`
  (goto _label))

(fn `UserConstructionScript`)