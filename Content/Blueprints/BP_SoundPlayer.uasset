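; BP_SoundPlayer is an actor that plays a configurable sound once, attached to its BoxTrigger component, with adjustable volume and attenuation.
; BeginPlay sets the ConditionSatisfied flag from AtStart, and Tick polls that flag, spawning the sound through a DoOnce when it is true.
; The graph has no overlap logic for the box, so without AtStart the sound waits until something external sets the flag.
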(event `self.ReceiveBeginPlay`
  (if (`self.AtStart`)
    (set `self.ConditionSatisfied` true)
    (else
      (set `self.ConditionSatisfied` false))))

(event `self.ReceiveTick`
  (params (DeltaSeconds :type "Float (single-precision)"))
  (if (`self.ConditionSatisfied`)
    (`/Engine/EditorBlueprintResources/StandardMacros.DoOnce` false
      (:`Completed`
        (`GameplayStatics.SpawnSoundAttached` (`self.SoundToPlay`) (`self.BoxTrigger`) "None" (0.0 0.0 0.0) (struct) "KeepRelativeOffset" false (`self.Volume`) 1.0 0.0 (`self.Sound Attenuation`) null)))))

(fn `UserConstructionScript`)