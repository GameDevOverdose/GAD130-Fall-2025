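; CCTV trigger Blueprint that drives a referenced Door actor between closed and opened heights.
; A Timeline lerps the door's Z, playing toward open on BeginPlay, which also enables CCTV, and when a BP_ShooterCharacter leaves the box trigger.
; Entering the trigger only casts the overlapping character.
; The Timeline reverse that would close the door for a valid character while CCTV is enabled is disconnected and never runs.
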(event `self.BoxTrigger.OnComponentBeginOverlap`
  (params (OverlappedComponent :type "PrimitiveComponent Object Reference") (OtherActor :type "Actor Object Reference") (OtherComp :type "PrimitiveComponent Object Reference") (OtherBodyIndex :type Integer) (bFromSweep :type Boolean) (SweepResult :type "HitResult Structure (by ref)"))
  ; CCTV Door Behavior
  (bind _output_get (set `self.Other Actor` OtherActor))
  (bind _asbp_shooter_character (cast `/Game/Variant_Shooter/Blueprints/BP_ShooterCharacter` _output_get)))

(event `self.ReceiveBeginPlay`
  (bind _door (`self.Door`))
  (bind (_returnvalue_x _returnvalue_y) (`KismetMathLibrary.BreakVector` (`self.K2_GetActorLocation` _door)))
  ; CCTV Door Behavior
  (`|ExecutionSequence`
    (:`then_0`
      (bind (_direction _value) (`Timeline|Timeline` :!label _label)
        (:`Update`
          (`self.K2_SetActorRelativeLocation` _door (`KismetMathLibrary.MakeVector` _returnvalue_x _returnvalue_y (`KismetMathLibrary.Lerp` (`self.ClosedZ`) (`self.OpenedZ`) _value)) false false))))
    (:`then_1`
      (set `self.CCTVEnabled` true))))

(event `self.BoxTrigger.OnComponentEndOverlap`
  (params (OverlappedComponent :type "PrimitiveComponent Object Reference") (OtherActor :type "Actor Object Reference") (OtherComp :type "PrimitiveComponent Object Reference") (OtherBodyIndex :type Integer))
  ; CCTV Door Behavior
  (bind _output_get (set `self.Other Actor` OtherActor))
  (cast `/Game/Variant_Shooter/Blueprints/BP_ShooterCharacter` _output_get)
  (goto _label))

(fn `UserConstructionScript`)